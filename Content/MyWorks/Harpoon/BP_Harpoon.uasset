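; BP_Harpoon is a grappling harpoon that pulls the player toward hook points.
; The Hook event traces along the camera's aim, storing the location of any BP_Hook_forHarpoon hit as the target.
; Tick first moves the visible cable to that target, then relaunches the character toward it every frame with LaunchCharacter.
; When the player gets close, it clears the state, hides the cable and returns it to the pawn.
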(event `Hook (Harpoon Shoot)`
  (bind _returnvalue (`GameplayStatics.GetPlayerCameraManager` 0))
  (if (`self.Is Attracting`)
    (bind (_outhit _returnvalue_2) (`KismetSystemLibrary.LineTraceSingle` :`Start` (`self.K2_GetActorLocation`) :`End` (+ (`PlayerCameraManager.GetCameraLocation` _returnvalue) (* (`self.GetActorForwardVector` _returnvalue) (`self.Harpoon Distance`))) :`TraceChannel` "TraceTypeQuery5" :`DrawDebugType` "ForOneFrame"))
    (if _returnvalue_2
      (bind _asbp_hook_for_harpoon (cast `/Game/MyWorks/Harpoon/BP_Hook_forHarpoon` (`.HitActor` (`GameplayStatics.BreakHitResult` _outhit)))
        (:`then`
          (set `self.Target` (`SceneComponent.K2_GetComponentLocation` (`Actor.RootComponent` _asbp_hook_for_harpoon)))
          (set `self.Is Attached` true))
        (:`CastFailed`
          (`KismetSystemLibrary.PrintString` "Cast Failed")))
      (else
        (`self.Stop Attraction`)))))

(event `self.ReceiveTick`
  (params (DeltaSeconds :type "Float (single-precision)"))
  (bind _cable (`self.Cable`))
  (if (`self.Is Attached`)
    (if (`self.Is Attraction Done`)
      (`self.Character Attraction`)
      (`SceneComponent.K2_SetWorldLocation` _cable (`KismetMathLibrary.VInterpTo` (`SceneComponent.K2_GetComponentLocation` _cable) (`self.Target`) (`GameplayStatics.GetWorldDeltaSeconds`) (`self.Cable Speed`)) false false)
      (`self.Stop Attraction`)
      (else
        (bind _is_attracted (`self.Pulling the cable`))
        (set `self.Is Attraction Done` _is_attracted)))))

(fn `Character Attraction`
  (bind _returnvalue (`GameplayStatics.GetPlayerCharacter` 0))
  (`Character.LaunchCharacter` _returnvalue (* (- (`self.Target`) (`self.K2_GetActorLocation` _returnvalue)) (* (`GameplayStatics.GetWorldDeltaSeconds`) (`self.Attraction Speed`))) true true)
  (return))

(fn `Pulling the cable`
  (returns (`Is Attracted` :type Boolean))
  (bind _target (`self.Target`))
  (bind _cable (`self.Cable`))
  (`SceneComponent.SetHiddenInGame` _cable false false)
  (if (<= (`KismetMathLibrary.VSize` (- (`SceneComponent.K2_GetComponentLocation` _cable) _target)) 100.0)
    (return true)
    (else
      (`SceneComponent.K2_SetWorldLocation` (`self.Cable`) (`KismetMathLibrary.VInterpTo` _target _target (`GameplayStatics.GetWorldDeltaSeconds`) (`self.Cable Speed`)) false false)
      (return false))))

(fn `Stop Attraction`
  (bind _cable (`self.Cable`))
  (if (<= (`KismetMathLibrary.Vector_Distance` (`self.Target`) (`self.K2_GetActorLocation` (`GameplayStatics.GetPlayerCharacter` 0))) 150.0)
    (set `self.Is Attached` false)
    (set `self.Is Attraction Done` false)
    (`SceneComponent.SetHiddenInGame` _cable true false)
    (`SceneComponent.K2_SetWorldLocation` _cable (`self.K2_GetActorLocation` (`GameplayStatics.GetPlayerPawn` 0)) false false)
    (return)))

(fn `UserConstructionScript`)