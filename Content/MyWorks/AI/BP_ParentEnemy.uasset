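; BP_ParentEnemy is a parent enemy pawn that handles taking damage and dying.
; AnyDamage subtracts from HP and prints the remaining value on screen.
; At zero HP it swaps the mesh material, prints a kill message, disables collision, stops the AI controller's brain logic and destroys itself after a death-animation delay.
; Its PawnSensing see-pawn event is an empty stub.
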(event `self.ReceiveAnyDamage`
  (params (Damage :type "Float (single-precision)") (DamageType :type "DamageType Object Reference") (InstigatedBy :type "Controller Object Reference") (DamageCauser :type "Actor Object Reference"))
  (bind _output_get (set `self.HP` (- (`self.HP`) Damage)))
  (`KismetSystemLibrary.PrintString` (`KismetStringLibrary.Conv_DoubleToString` _output_get) true true (struct :`G` 1.0 :`B` 0.242281 :`A` 1.0))
  (if (<= (`self.HP`) 0.0)
    (`PrimitiveComponent.SetMaterial` (`self.Mesh`) 0 (`self.Material`))
    (`KismetSystemLibrary.PrintString` (`self.EnemyKilled Text`) true true (struct :`G` 1.0 :`B` 0.242281 :`A` 1.0))
    (`self.SetActorEnableCollision` false)
    (`BrainComponent.StopLogic` (`AIController.BrainComponent` (`AIBlueprintHelperLibrary.GetAIController` self)) "Smertb")
    (`KismetSystemLibrary.Delay` (`self.DeathAnimation Duration`))
    (`self.K2_DestroyActor`)))

(event `self.PawnSensing.OnSeePawn`
  (params (Pawn :type "Pawn Object Reference")))

(fn `UserConstructionScript`)