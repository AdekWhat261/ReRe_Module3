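; Behavior tree task that makes a Ram AI charge the player and deal area damage on impact.
; It triples the ram's max walk speed without restoring it, then uses AIMoveTo to chase the player character.
; On reaching the player it applies radial damage around itself and finishes successfully.
; A failed move or cast never finishes the task.
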(event `self.ReceiveExecuteAI`
  (params (OwnerController :type "AIController Object Reference") (ControlledPawn :type "Pawn Object Reference"))
  (bind _asbp_ram (cast `/Game/MyWorks/AI/Ram/BP_Ram` ControlledPawn))
  (bind _charactermovement (`Character.CharacterMovement` _asbp_ram))
  (set `CharacterMovementComponent.MaxWalkSpeed` (* (`CharacterMovementComponent.MaxWalkSpeed` _charactermovement) 3.0) _charactermovement)
  (`|AIMoveTo` ControlledPawn (0.0 0.0 0.0) (`GameplayStatics.GetPlayerCharacter` 0) 10.0
    (:`OnSuccess`
      (`GameplayStatics.ApplyRadialDamage` :`BaseDamage` (`self.DMG`) :`Origin` (`Actor.K2_GetActorLocation` ControlledPawn) :`DamageRadius` (`self.Damage Radius`) :`DamageCauser` _asbp_ram :`InstigatedByController` OwnerController :`DamagePreventionChannel` "ECC_GameTraceChannel2")
      (`self.FinishExecute` true))))