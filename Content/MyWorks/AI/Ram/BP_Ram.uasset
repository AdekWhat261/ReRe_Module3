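; BP_Ram is an AI battering ram that moves to a breach point once a trigger is activated.
; Each tick it looks up the TriggerBox actor in the level with GetActorOfClass and checks its IsTriggered flag.
; While that flag is set, it calls AIMoveTo through RamsController toward the BreakinPoint goal actor, re-issuing the move every frame.
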(event `self.ReceiveBeginPlay`
  (`parent.ReceiveBeginPlay`))

(event `self.ReceiveTick`
  (params (DeltaSeconds :type "Float (single-precision)"))
  (bind _returnvalue (`GameplayStatics.GetActorOfClass` (`self.TriggerBox`)))
  (if (`/Game/MyWorks/AI/Ram/BP_RamTriggerBox.IsTriggered` _returnvalue)
    (`AITask_MoveTo.AIMoveTo` (`self.Ram's Controller`) (0.0 0.0 0.0) (`self.Break-in Point`))))

(fn `UserConstructionScript`
  (`parent.UserConstructionScript`))