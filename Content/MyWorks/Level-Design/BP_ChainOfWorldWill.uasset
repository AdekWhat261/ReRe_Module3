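; BP_ChainOfWorldWill is a damageable chain actor meant to be one of a set the player destroys.
; Any damage lowers HP; at zero or below it prints a kill message, waits out a death-animation delay and destroys itself.
; On Destroyed it increments its own clamped DestroyedChainsCount and prints a completion message when that equals AllChainsCount.
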(event `self.ReceiveAnyDamage`
  (params (Damage :type "Float (single-precision)") (DamageType :type "DamageType Object Reference") (InstigatedBy :type "Controller Object Reference") (DamageCauser :type "Actor Object Reference"))
  (bind _output_get (set `self.HP` (- (`self.HP`) Damage)))
  (`KismetSystemLibrary.PrintString` (`KismetStringLibrary.Conv_DoubleToString` _output_get) true true (struct :`A` 1.0))
  (if (<= (`self.HP`) 0.0)
    (`KismetSystemLibrary.PrintString` (`self.[Enemy's Name] Was Killed!`) true true (struct :`A` 1.0))
    (`KismetSystemLibrary.Delay` (`self.Duration of Death Animation`))
    (`self.K2_DestroyActor`)))

(event `self.ReceiveDestroyed`
  ;[0.01389 0.01389 0.01389] Chains destroying System
  (set `self.Destroyed chains' count` (`KismetMathLibrary.Clamp` (+ (`self.Destroyed chains' count`) 1) 0 (`self.All chains' count`)))
  (`self.AllChains Destroyed`))

(event `AllChains Destroyed`
  ;[0.01389 0.01389 0.01389] Chains destroying System
  (if (== (`self.Destroyed chains' count`) (`self.All chains' count`))
    (`KismetSystemLibrary.PrintString` "You've Destroyed all Chains! Tu-du-Duu" true true (struct :`G` 0.101539 :`B` 1.0 :`A` 1.0) 5.0)))

(fn `UserConstructionScript`)